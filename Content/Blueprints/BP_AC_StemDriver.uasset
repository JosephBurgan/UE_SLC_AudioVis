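; Component that drives material parameters from the individual stems of a MetaSound music track.
; StartMusic plays the music audio quantized to the beat on a Quartz clock, then watches one MetaSound output per stem, from bass and drums to pads and effects.
; Each output change writes its float to the matching Stem_ scalar in MPC_ParameterCollection, letting materials react to each stem.
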(event Custom|MusicStarted
  (params (EventType :type EQuartzCommandDelegateSubType%20Enum :default "CommandOnFailedToQueue") (Name :type Name)))

(event Custom|OnPadsChanged
  (params (OutputName :type Name) (Output :type Meta%20Sound%20Output%20Structure%20%28by%20ref%29))
  (bind _returnvalue (Class|MetasoundOutputBlueprintAccess|GetFloat Output))
  (Rendering|Material|SetScalarParameterValue "/Game/Materials/MPC_ParameterCollection.MPC_ParameterCollection" "Stem_Pads" _returnvalue :!class /Script/Engine.KismetMaterialLibrary))

(event Custom|OnPlucksChanged
  (params (OutputName :type Name) (Output :type Meta%20Sound%20Output%20Structure%20%28by%20ref%29))
  (bind _returnvalue (Class|MetasoundOutputBlueprintAccess|GetFloat Output))
  (Rendering|Material|SetScalarParameterValue "/Game/Materials/MPC_ParameterCollection.MPC_ParameterCollection" "Stem_Plucks" _returnvalue :!class /Script/Engine.KismetMaterialLibrary))

(event Custom|OnBassChanged
  (params (OutputName :type Name) (Output :type Meta%20Sound%20Output%20Structure%20%28by%20ref%29))
  (bind _returnvalue (Class|MetasoundOutputBlueprintAccess|GetFloat Output))
  (Rendering|Material|SetScalarParameterValue "/Game/Materials/MPC_ParameterCollection.MPC_ParameterCollection" "Stem_Bass" _returnvalue :!class /Script/Engine.KismetMaterialLibrary))

(event Custom|StartMusic
  (bind _returnvalue (WorldSubsystems|GetMetaSoundOutputSubsystem))
  (bind _musicaudio (Variables|Default|GetMusicAudio))
  (Audio|Components|Audio|PlayQuantized (Variables|Default|GetMusicAudio) (Variables|Default|GetQuartzClock) (Utilities|Struct|MakeQuartzQuantizationBoundary "Beat" 1.0 "BarRelative" true false false false) 0)
  (MetaSoundOutput|WatchOutput _returnvalue _musicaudio "Bass" (delegate Custom|OnBassChanged) "None" "None" :!class /Script/MetasoundEngine.MetaSoundOutputSubsystem)
  (MetaSoundOutput|WatchOutput _returnvalue _musicaudio "Chords" (delegate Custom|OnChordsChanged) "None" "None" :!class /Script/MetasoundEngine.MetaSoundOutputSubsystem)
  (MetaSoundOutput|WatchOutput _returnvalue _musicaudio "Drums" (delegate Custom|OnDrumsChanged) "None" "None" :!class /Script/MetasoundEngine.MetaSoundOutputSubsystem)
  (MetaSoundOutput|WatchOutput _returnvalue _musicaudio "FXGameBoy" (delegate Custom|OnFXGameBoyChanged) "None" "None" :!class /Script/MetasoundEngine.MetaSoundOutputSubsystem)
  (MetaSoundOutput|WatchOutput _returnvalue _musicaudio "FXGrowls" (delegate Custom|OnFXGrowlsChanged) "None" "None" :!class /Script/MetasoundEngine.MetaSoundOutputSubsystem)
  (MetaSoundOutput|WatchOutput _returnvalue _musicaudio "Lead" (delegate Custom|OnLeadChanged) "None" "None" :!class /Script/MetasoundEngine.MetaSoundOutputSubsystem)
  (MetaSoundOutput|WatchOutput _returnvalue _musicaudio "Pads" (delegate Custom|OnPadsChanged) "None" "None" :!class /Script/MetasoundEngine.MetaSoundOutputSubsystem)
  (MetaSoundOutput|WatchOutput _returnvalue _musicaudio "Plucks" (delegate Custom|OnPlucksChanged) "None" "None" :!class /Script/MetasoundEngine.MetaSoundOutputSubsystem))

(event Custom|OnChordsChanged
  (params (OutputName :type Name) (Output :type Meta%20Sound%20Output%20Structure%20%28by%20ref%29))
  (bind _returnvalue (Class|MetasoundOutputBlueprintAccess|GetFloat Output))
  (Rendering|Material|SetScalarParameterValue "/Game/Materials/MPC_ParameterCollection.MPC_ParameterCollection" "Stem_Chords" _returnvalue :!class /Script/Engine.KismetMaterialLibrary))

(event Custom|OnDrumsChanged
  (params (OutputName :type Name) (Output :type Meta%20Sound%20Output%20Structure%20%28by%20ref%29))
  (bind _returnvalue (Class|MetasoundOutputBlueprintAccess|GetFloat Output))
  (Rendering|Material|SetScalarParameterValue "/Game/Materials/MPC_ParameterCollection.MPC_ParameterCollection" "Stem_Drums" _returnvalue :!class /Script/Engine.KismetMaterialLibrary))

(event Custom|OnFXGameBoyChanged
  (params (OutputName :type Name) (Output :type Meta%20Sound%20Output%20Structure%20%28by%20ref%29))
  (bind _returnvalue (Class|MetasoundOutputBlueprintAccess|GetFloat Output))
  (Rendering|Material|SetScalarParameterValue "/Game/Materials/MPC_ParameterCollection.MPC_ParameterCollection" "Stem_FXGameBoy" _returnvalue :!class /Script/Engine.KismetMaterialLibrary))

(event Custom|OnFXGrowlsChanged
  (params (OutputName :type Name) (Output :type Meta%20Sound%20Output%20Structure%20%28by%20ref%29))
  (bind _returnvalue (Class|MetasoundOutputBlueprintAccess|GetFloat Output))
  (Rendering|Material|SetScalarParameterValue "/Game/Materials/MPC_ParameterCollection.MPC_ParameterCollection" "Stem_FXGrowls" _returnvalue :!class /Script/Engine.KismetMaterialLibrary))

(event Custom|OnLeadChanged
  (params (OutputName :type Name) (Output :type Meta%20Sound%20Output%20Structure%20%28by%20ref%29))
  (bind _returnvalue (Class|MetasoundOutputBlueprintAccess|GetFloat Output))
  (Rendering|Material|SetScalarParameterValue "/Game/Materials/MPC_ParameterCollection.MPC_ParameterCollection" "Stem_Lead" _returnvalue :!class /Script/Engine.KismetMaterialLibrary))

(event EventBeginPlay)

(event EventTick
  (params (DeltaSeconds :type Float%20%28single-precision%29)))
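; Beat manager actor that drives materials from music timing and stem analysis through a Material Parameter Collection.
; BeginPlay creates a Quartz clock at the set BPM and starts it after a short delay.
; Each quarter note plays a beep and writes the beat number, while Tick writes beat progress.
; When music is enabled, it plays stems quantized and watches MetaSound outputs, copying per-stem and low/mid/high band values into the collection.
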(event Custom|Set%20StemDriver%20Variables)

(event Custom|Beat
  (params (ClockName :type Name) (QuantizationType :type EQuartzCommandQuantization%20Enum :default "Bar") (NumBars :type Integer) (Beat :type Integer) (BeatFraction :type Float%20%28single-precision%29))
  ;[0.15 0.15 0.15 0.5] 4.
  ; - "Subsribe to Quantization Event"
  ; - Change Quantezation Enum
  ; - Drag off Red pin and make Custom Event
  ;[0.15 0.15 0.15 0.5] 5.
  ; - Make a Material Parameter Collection asset in the Content Browser
  ; - Add a Scalar Parameter and name it
  ; - Add this "Set Scalar Paramter Value" node
  ; - Set Collection as your Material Paramter Collection asset
  ; - Select the Parameter Name
  ; - Input the Beat Fraction
  (Rendering|Material|SetScalarParameterValue "/Game/Materials/MPC_ParameterCollection.MPC_ParameterCollection" "Beat" (Math|Conversions|ToFloat(Integer) Beat) :!class /Script/Engine.KismetMaterialLibrary)
  ;[0.15 0.15 0.15 0.5] 6.
  ; - Play MetaSound asset "BeepTone"
  (Audio|Components|Audio|Play (Variables|Default|GetAudioComp%20MS_BeepTone) 0.0))

(event Custom|OnPadsChanged
  (params (OutputName :type Name) (Output :type Meta%20Sound%20Output%20Structure%20%28by%20ref%29))
  (bind _returnvalue (Class|MetasoundOutputBlueprintAccess|GetFloat Output))
  (Rendering|Material|SetScalarParameterValue "/Game/Materials/MPC_ParameterCollection.MPC_ParameterCollection" "Pads_Stem" _returnvalue :!class /Script/Engine.KismetMaterialLibrary))

(event Custom|OnPlucksChanged
  (params (OutputName :type Name) (Output :type Meta%20Sound%20Output%20Structure%20%28by%20ref%29))
  (bind _returnvalue (Class|MetasoundOutputBlueprintAccess|GetFloat Output))
  (Rendering|Material|SetScalarParameterValue "/Game/Materials/MPC_ParameterCollection.MPC_ParameterCollection" "Plucks_Stem" _returnvalue :!class /Script/Engine.KismetMaterialLibrary))

(event Custom|OnBassLowChanged
  (params (OutputName :type Name) (Output :type Meta%20Sound%20Output%20Structure%20%28by%20ref%29))
  (bind _returnvalue (Class|MetasoundOutputBlueprintAccess|GetFloat Output))
  (Rendering|Material|SetScalarParameterValue "/Game/Materials/MPC_ParameterCollection.MPC_ParameterCollection" "BassLow" _returnvalue :!class /Script/Engine.KismetMaterialLibrary))

(event Custom|OnBassMidChanged
  (params (OutputName :type Name) (Output :type Meta%20Sound%20Output%20Structure%20%28by%20ref%29))
  (bind _returnvalue (Class|MetasoundOutputBlueprintAccess|GetFloat Output))
  (Rendering|Material|SetScalarParameterValue "/Game/Materials/MPC_ParameterCollection.MPC_ParameterCollection" "BassMid" _returnvalue :!class /Script/Engine.KismetMaterialLibrary))

(event Custom|OnBassHighChanged
  (params (OutputName :type Name) (Output :type Meta%20Sound%20Output%20Structure%20%28by%20ref%29))
  (bind _returnvalue (Class|MetasoundOutputBlueprintAccess|GetFloat Output))
  (Rendering|Material|SetScalarParameterValue "/Game/Materials/MPC_ParameterCollection.MPC_ParameterCollection" "BassHigh" _returnvalue :!class /Script/Engine.KismetMaterialLibrary))

(event Custom|OnChordsLowChanged
  (params (OutputName :type Name) (Output :type Meta%20Sound%20Output%20Structure%20%28by%20ref%29))
  (bind _returnvalue (Class|MetasoundOutputBlueprintAccess|GetFloat Output))
  (Rendering|Material|SetScalarParameterValue "/Game/Materials/MPC_ParameterCollection.MPC_ParameterCollection" "ChordsLow" _returnvalue :!class /Script/Engine.KismetMaterialLibrary))

(event Custom|OnChordsMidChanged
  (params (OutputName :type Name) (Output :type Meta%20Sound%20Output%20Structure%20%28by%20ref%29))
  (bind _returnvalue (Class|MetasoundOutputBlueprintAccess|GetFloat Output))
  (Rendering|Material|SetScalarParameterValue "/Game/Materials/MPC_ParameterCollection.MPC_ParameterCollection" "ChordsMid" _returnvalue :!class /Script/Engine.KismetMaterialLibrary))

(event Custom|OnChordsHighChanged
  (params (OutputName :type Name) (Output :type Meta%20Sound%20Output%20Structure%20%28by%20ref%29))
  (bind _returnvalue (Class|MetasoundOutputBlueprintAccess|GetFloat Output))
  (Rendering|Material|SetScalarParameterValue "/Game/Materials/MPC_ParameterCollection.MPC_ParameterCollection" "ChordsHigh" _returnvalue :!class /Script/Engine.KismetMaterialLibrary))

(event Custom|OnDrumsLowChanged
  (params (OutputName :type Name) (Output :type Meta%20Sound%20Output%20Structure%20%28by%20ref%29))
  (bind _returnvalue (Class|MetasoundOutputBlueprintAccess|GetFloat Output))
  (Rendering|Material|SetScalarParameterValue "/Game/Materials/MPC_ParameterCollection.MPC_ParameterCollection" "DrumsLow" _returnvalue :!class /Script/Engine.KismetMaterialLibrary))

(event Custom|OnBassChanged
  (params (OutputName :type Name) (Output :type Meta%20Sound%20Output%20Structure%20%28by%20ref%29))
  (bind _returnvalue (Class|MetasoundOutputBlueprintAccess|GetFloat Output))
  (Rendering|Material|SetScalarParameterValue "/Game/Materials/MPC_ParameterCollection.MPC_ParameterCollection" "Bass_Stem" _returnvalue :!class /Script/Engine.KismetMaterialLibrary))

(event Custom|OnDrumsMidChanged
  (params (OutputName :type Name) (Output :type Meta%20Sound%20Output%20Structure%20%28by%20ref%29))
  (bind _returnvalue (Class|MetasoundOutputBlueprintAccess|GetFloat Output))
  (Rendering|Material|SetScalarParameterValue "/Game/Materials/MPC_ParameterCollection.MPC_ParameterCollection" "DrumsMid" _returnvalue :!class /Script/Engine.KismetMaterialLibrary))

(event Custom|OnDrumsHighChanged
  (params (OutputName :type Name) (Output :type Meta%20Sound%20Output%20Structure%20%28by%20ref%29))
  (bind _returnvalue (Class|MetasoundOutputBlueprintAccess|GetFloat Output))
  (Rendering|Material|SetScalarParameterValue "/Game/Materials/MPC_ParameterCollection.MPC_ParameterCollection" "DrumsHigh" _returnvalue :!class /Script/Engine.KismetMaterialLibrary))

(event Custom|OnFXGameBoyLowChanged
  (params (OutputName :type Name) (Output :type Meta%20Sound%20Output%20Structure%20%28by%20ref%29))
  (bind _returnvalue (Class|MetasoundOutputBlueprintAccess|GetFloat Output))
  (Rendering|Material|SetScalarParameterValue "/Game/Materials/MPC_ParameterCollection.MPC_ParameterCollection" "FXGameBoyLow" _returnvalue :!class /Script/Engine.KismetMaterialLibrary))

(event Custom|OnFXGameBoyMidChanged
  (params (OutputName :type Name) (Output :type Meta%20Sound%20Output%20Structure%20%28by%20ref%29))
  (bind _returnvalue (Class|MetasoundOutputBlueprintAccess|GetFloat Output))
  (Rendering|Material|SetScalarParameterValue "/Game/Materials/MPC_ParameterCollection.MPC_ParameterCollection" "FXGameBoyMid" _returnvalue :!class /Script/Engine.KismetMaterialLibrary))

(event Custom|OnFXGameBoyHighChanged
  (params (OutputName :type Name) (Output :type Meta%20Sound%20Output%20Structure%20%28by%20ref%29))
  (bind _returnvalue (Class|MetasoundOutputBlueprintAccess|GetFloat Output))
  (Rendering|Material|SetScalarParameterValue "/Game/Materials/MPC_ParameterCollection.MPC_ParameterCollection" "FXGameBoyHigh" _returnvalue :!class /Script/Engine.KismetMaterialLibrary))

(event Custom|OnFXGrowlsLowChanged
  (params (OutputName :type Name) (Output :type Meta%20Sound%20Output%20Structure%20%28by%20ref%29))
  (bind _returnvalue (Class|MetasoundOutputBlueprintAccess|GetFloat Output))
  (Rendering|Material|SetScalarParameterValue "/Game/Materials/MPC_ParameterCollection.MPC_ParameterCollection" "FXGrowlsLow" _returnvalue :!class /Script/Engine.KismetMaterialLibrary))

(event Custom|OnFXGrowlsMidChanged
  (params (OutputName :type Name) (Output :type Meta%20Sound%20Output%20Structure%20%28by%20ref%29))
  (bind _returnvalue (Class|MetasoundOutputBlueprintAccess|GetFloat Output))
  (Rendering|Material|SetScalarParameterValue "/Game/Materials/MPC_ParameterCollection.MPC_ParameterCollection" "FXGrowlsMid" _returnvalue :!class /Script/Engine.KismetMaterialLibrary))

(event Custom|OnFXGrowlsHighChanged
  (params (OutputName :type Name) (Output :type Meta%20Sound%20Output%20Structure%20%28by%20ref%29))
  (bind _returnvalue (Class|MetasoundOutputBlueprintAccess|GetFloat Output))
  (Rendering|Material|SetScalarParameterValue "/Game/Materials/MPC_ParameterCollection.MPC_ParameterCollection" "FXGrowlsHigh" _returnvalue :!class /Script/Engine.KismetMaterialLibrary))

(event Custom|OnLeadLowChanged
  (params (OutputName :type Name) (Output :type Meta%20Sound%20Output%20Structure%20%28by%20ref%29))
  (bind _returnvalue (Class|MetasoundOutputBlueprintAccess|GetFloat Output))
  (Rendering|Material|SetScalarParameterValue "/Game/Materials/MPC_ParameterCollection.MPC_ParameterCollection" "LeadLow" _returnvalue :!class /Script/Engine.KismetMaterialLibrary))

(event Custom|OnLeadMidChanged
  (params (OutputName :type Name) (Output :type Meta%20Sound%20Output%20Structure%20%28by%20ref%29))
  (bind _returnvalue (Class|MetasoundOutputBlueprintAccess|GetFloat Output))
  (Rendering|Material|SetScalarParameterValue "/Game/Materials/MPC_ParameterCollection.MPC_ParameterCollection" "LeadMid" _returnvalue :!class /Script/Engine.KismetMaterialLibrary))

(event Custom|Start%20Music
  (Audio|Components|Audio|PlayQuantized (Variables|Default|GetAudioComp%20Stems) (Variables|Default|GetQuartzClockHandle) (Utilities|Struct|MakeQuartzQuantizationBoundary "Beat" 1.0 "BarRelative" true false false false) 0)
  (Utilities|FlowControl|Sequence
    (:then_0
      (MetaSoundOutput|WatchOutput (WorldSubsystems|GetMetaSoundOutputSubsystem) (Variables|Default|GetAudioComp%20Stems) "Bass" (delegate Custom|OnBassChanged) "None" "None" :!class /Script/MetasoundEngine.MetaSoundOutputSubsystem)
      (MetaSoundOutput|WatchOutput (WorldSubsystems|GetMetaSoundOutputSubsystem) (Variables|Default|GetAudioComp%20Stems) "BassLow" (delegate Custom|OnBassLowChanged) "None" "None" :!class /Script/MetasoundEngine.MetaSoundOutputSubsystem)
      (MetaSoundOutput|WatchOutput (WorldSubsystems|GetMetaSoundOutputSubsystem) (Variables|Default|GetAudioComp%20Stems) "BassMid" (delegate Custom|OnBassMidChanged) "None" "None" :!class /Script/MetasoundEngine.MetaSoundOutputSubsystem)
      (MetaSoundOutput|WatchOutput (WorldSubsystems|GetMetaSoundOutputSubsystem) (Variables|Default|GetAudioComp%20Stems) "BassHigh" (delegate Custom|OnBassHighChanged) "None" "None" :!class /Script/MetasoundEngine.MetaSoundOutputSubsystem))
    (:then_1
      (MetaSoundOutput|WatchOutput (WorldSubsystems|GetMetaSoundOutputSubsystem) (Variables|Default|GetAudioComp%20Stems) "Chords" (delegate Custom|OnChordsChanged) "None" "None" :!class /Script/MetasoundEngine.MetaSoundOutputSubsystem)
      (MetaSoundOutput|WatchOutput (WorldSubsystems|GetMetaSoundOutputSubsystem) (Variables|Default|GetAudioComp%20Stems) "ChordsLow" (delegate Custom|OnChordsLowChanged) "None" "None" :!class /Script/MetasoundEngine.MetaSoundOutputSubsystem)
      (MetaSoundOutput|WatchOutput (WorldSubsystems|GetMetaSoundOutputSubsystem) (Variables|Default|GetAudioComp%20Stems) "ChordsMid" (delegate Custom|OnChordsMidChanged) "None" "None" :!class /Script/MetasoundEngine.MetaSoundOutputSubsystem)
      (MetaSoundOutput|WatchOutput (WorldSubsystems|GetMetaSoundOutputSubsystem) (Variables|Default|GetAudioComp%20Stems) "ChordsHigh" (delegate Custom|OnChordsHighChanged) "None" "None" :!class /Script/MetasoundEngine.MetaSoundOutputSubsystem))
    (:then_2
      (MetaSoundOutput|WatchOutput (WorldSubsystems|GetMetaSoundOutputSubsystem) (Variables|Default|GetAudioComp%20Stems) "Drums" (delegate Custom|OnDrumsChanged) "None" "None" :!class /Script/MetasoundEngine.MetaSoundOutputSubsystem)
      (MetaSoundOutput|WatchOutput (WorldSubsystems|GetMetaSoundOutputSubsystem) (Variables|Default|GetAudioComp%20Stems) "DrumsLow" (delegate Custom|OnDrumsLowChanged) "None" "None" :!class /Script/MetasoundEngine.MetaSoundOutputSubsystem)
      (MetaSoundOutput|WatchOutput (WorldSubsystems|GetMetaSoundOutputSubsystem) (Variables|Default|GetAudioComp%20Stems) "DrumsMid" (delegate Custom|OnDrumsMidChanged) "None" "None" :!class /Script/MetasoundEngine.MetaSoundOutputSubsystem)
      (MetaSoundOutput|WatchOutput (WorldSubsystems|GetMetaSoundOutputSubsystem) (Variables|Default|GetAudioComp%20Stems) "DrumsHigh" (delegate Custom|OnDrumsHighChanged) "None" "None" :!class /Script/MetasoundEngine.MetaSoundOutputSubsystem))
    (:then_3
      (MetaSoundOutput|WatchOutput (WorldSubsystems|GetMetaSoundOutputSubsystem) (Variables|Default|GetAudioComp%20Stems) "FXGameBoy" (delegate Custom|OnFXGameBoyChanged) "None" "None" :!class /Script/MetasoundEngine.MetaSoundOutputSubsystem)
      (MetaSoundOutput|WatchOutput (WorldSubsystems|GetMetaSoundOutputSubsystem) (Variables|Default|GetAudioComp%20Stems) "FXGameBoyLow" (delegate Custom|OnFXGameBoyLowChanged) "None" "None" :!class /Script/MetasoundEngine.MetaSoundOutputSubsystem)
      (MetaSoundOutput|WatchOutput (WorldSubsystems|GetMetaSoundOutputSubsystem) (Variables|Default|GetAudioComp%20Stems) "FXGameBoyMid" (delegate Custom|OnFXGameBoyMidChanged) "None" "None" :!class /Script/MetasoundEngine.MetaSoundOutputSubsystem)
      (MetaSoundOutput|WatchOutput (WorldSubsystems|GetMetaSoundOutputSubsystem) (Variables|Default|GetAudioComp%20Stems) "FXGameBoyHigh" (delegate Custom|OnFXGameBoyHighChanged) "None" "None" :!class /Script/MetasoundEngine.MetaSoundOutputSubsystem))
    (:then_4
      (MetaSoundOutput|WatchOutput (WorldSubsystems|GetMetaSoundOutputSubsystem) (Variables|Default|GetAudioComp%20Stems) "FXGrowls" (delegate Custom|OnFXGrowlsChanged) "None" "None" :!class /Script/MetasoundEngine.MetaSoundOutputSubsystem)
      (MetaSoundOutput|WatchOutput (WorldSubsystems|GetMetaSoundOutputSubsystem) (Variables|Default|GetAudioComp%20Stems) "FXGrowlsLow" (delegate Custom|OnFXGrowlsLowChanged) "None" "None" :!class /Script/MetasoundEngine.MetaSoundOutputSubsystem)
      (MetaSoundOutput|WatchOutput (WorldSubsystems|GetMetaSoundOutputSubsystem) (Variables|Default|GetAudioComp%20Stems) "FXGrowlsMid" (delegate Custom|OnFXGrowlsMidChanged) "None" "None" :!class /Script/MetasoundEngine.MetaSoundOutputSubsystem)
      (MetaSoundOutput|WatchOutput (WorldSubsystems|GetMetaSoundOutputSubsystem) (Variables|Default|GetAudioComp%20Stems) "FXGrowlsHigh" (delegate Custom|OnFXGrowlsHighChanged) "None" "None" :!class /Script/MetasoundEngine.MetaSoundOutputSubsystem))
    (:then_5
      (MetaSoundOutput|WatchOutput (WorldSubsystems|GetMetaSoundOutputSubsystem) (Variables|Default|GetAudioComp%20Stems) "Lead" (delegate Custom|OnLeadChanged) "None" "None" :!class /Script/MetasoundEngine.MetaSoundOutputSubsystem)
      (MetaSoundOutput|WatchOutput (WorldSubsystems|GetMetaSoundOutputSubsystem) (Variables|Default|GetAudioComp%20Stems) "LeadLow" (delegate Custom|OnLeadLowChanged) "None" "None" :!class /Script/MetasoundEngine.MetaSoundOutputSubsystem)
      (MetaSoundOutput|WatchOutput (WorldSubsystems|GetMetaSoundOutputSubsystem) (Variables|Default|GetAudioComp%20Stems) "LeadMid" (delegate Custom|OnLeadMidChanged) "None" "None" :!class /Script/MetasoundEngine.MetaSoundOutputSubsystem)
      (MetaSoundOutput|WatchOutput (WorldSubsystems|GetMetaSoundOutputSubsystem) (Variables|Default|GetAudioComp%20Stems) "LeadHigh" (delegate Custom|OnLeadHighChanged) "None" "None" :!class /Script/MetasoundEngine.MetaSoundOutputSubsystem))
    (:then_6
      (MetaSoundOutput|WatchOutput (WorldSubsystems|GetMetaSoundOutputSubsystem) (Variables|Default|GetAudioComp%20Stems) "Pads" (delegate Custom|OnPadsChanged) "None" "None" :!class /Script/MetasoundEngine.MetaSoundOutputSubsystem)
      (MetaSoundOutput|WatchOutput (WorldSubsystems|GetMetaSoundOutputSubsystem) (Variables|Default|GetAudioComp%20Stems) "PadsLow" (delegate Custom|OnPadsLowChanged) "None" "None" :!class /Script/MetasoundEngine.MetaSoundOutputSubsystem)
      (MetaSoundOutput|WatchOutput (WorldSubsystems|GetMetaSoundOutputSubsystem) (Variables|Default|GetAudioComp%20Stems) "PadsMid" (delegate Custom|OnPadsMidChanged) "None" "None" :!class /Script/MetasoundEngine.MetaSoundOutputSubsystem)
      (MetaSoundOutput|WatchOutput (WorldSubsystems|GetMetaSoundOutputSubsystem) (Variables|Default|GetAudioComp%20Stems) "PadsHigh" (delegate Custom|OnPadsHighChanged) "None" "None" :!class /Script/MetasoundEngine.MetaSoundOutputSubsystem))
    (:then_7
      (MetaSoundOutput|WatchOutput (WorldSubsystems|GetMetaSoundOutputSubsystem) (Variables|Default|GetAudioComp%20Stems) "Plucks" (delegate Custom|OnPlucksChanged) "None" "None" :!class /Script/MetasoundEngine.MetaSoundOutputSubsystem)
      (MetaSoundOutput|WatchOutput (WorldSubsystems|GetMetaSoundOutputSubsystem) (Variables|Default|GetAudioComp%20Stems) "PlucksLow" (delegate Custom|OnPlucksLowChanged) "None" "None" :!class /Script/MetasoundEngine.MetaSoundOutputSubsystem)
      (MetaSoundOutput|WatchOutput (WorldSubsystems|GetMetaSoundOutputSubsystem) (Variables|Default|GetAudioComp%20Stems) "PlucksMid" (delegate Custom|OnPlucksMidChanged) "None" "None" :!class /Script/MetasoundEngine.MetaSoundOutputSubsystem)
      (MetaSoundOutput|WatchOutput (WorldSubsystems|GetMetaSoundOutputSubsystem) (Variables|Default|GetAudioComp%20Stems) "PlucksHigh" (delegate Custom|OnPlucksHighChanged) "None" "None" :!class /Script/MetasoundEngine.MetaSoundOutputSubsystem))))

(event Custom|OnLeadHighChanged
  (params (OutputName :type Name) (Output :type Meta%20Sound%20Output%20Structure%20%28by%20ref%29))
  (bind _returnvalue (Class|MetasoundOutputBlueprintAccess|GetFloat Output))
  (Rendering|Material|SetScalarParameterValue "/Game/Materials/MPC_ParameterCollection.MPC_ParameterCollection" "LeadHigh" _returnvalue :!class /Script/Engine.KismetMaterialLibrary))

(event Custom|OnPadsLowChanged
  (params (OutputName :type Name) (Output :type Meta%20Sound%20Output%20Structure%20%28by%20ref%29))
  (bind _returnvalue (Class|MetasoundOutputBlueprintAccess|GetFloat Output))
  (Rendering|Material|SetScalarParameterValue "/Game/Materials/MPC_ParameterCollection.MPC_ParameterCollection" "PadsLow" _returnvalue :!class /Script/Engine.KismetMaterialLibrary))

(event Custom|OnPlucksLowChanged
  (params (OutputName :type Name) (Output :type Meta%20Sound%20Output%20Structure%20%28by%20ref%29))
  (bind _returnvalue (Class|MetasoundOutputBlueprintAccess|GetFloat Output))
  (Rendering|Material|SetScalarParameterValue "/Game/Materials/MPC_ParameterCollection.MPC_ParameterCollection" "PlucksLow" _returnvalue :!class /Script/Engine.KismetMaterialLibrary))

(event Custom|OnPadsMidChanged
  (params (OutputName :type Name) (Output :type Meta%20Sound%20Output%20Structure%20%28by%20ref%29))
  (bind _returnvalue (Class|MetasoundOutputBlueprintAccess|GetFloat Output))
  (Rendering|Material|SetScalarParameterValue "/Game/Materials/MPC_ParameterCollection.MPC_ParameterCollection" "PadsMid" _returnvalue :!class /Script/Engine.KismetMaterialLibrary))

(event Custom|OnPadsHighChanged
  (params (OutputName :type Name) (Output :type Meta%20Sound%20Output%20Structure%20%28by%20ref%29))
  (bind _returnvalue (Class|MetasoundOutputBlueprintAccess|GetFloat Output))
  (Rendering|Material|SetScalarParameterValue "/Game/Materials/MPC_ParameterCollection.MPC_ParameterCollection" "PadsHigh" _returnvalue :!class /Script/Engine.KismetMaterialLibrary))

(event Custom|OnPlucksHighChanged
  (params (OutputName :type Name) (Output :type Meta%20Sound%20Output%20Structure%20%28by%20ref%29))
  (bind _returnvalue (Class|MetasoundOutputBlueprintAccess|GetFloat Output))
  (Rendering|Material|SetScalarParameterValue "/Game/Materials/MPC_ParameterCollection.MPC_ParameterCollection" "PlucksHigh" _returnvalue :!class /Script/Engine.KismetMaterialLibrary))

(event Custom|OnPlucksMidChanged
  (params (OutputName :type Name) (Output :type Meta%20Sound%20Output%20Structure%20%28by%20ref%29))
  (bind _returnvalue (Class|MetasoundOutputBlueprintAccess|GetFloat Output))
  (Rendering|Material|SetScalarParameterValue "/Game/Materials/MPC_ParameterCollection.MPC_ParameterCollection" "PlucksMid" _returnvalue :!class /Script/Engine.KismetMaterialLibrary))

(event Custom|OnChordsChanged
  (params (OutputName :type Name) (Output :type Meta%20Sound%20Output%20Structure%20%28by%20ref%29))
  (bind _returnvalue (Class|MetasoundOutputBlueprintAccess|GetFloat Output))
  (Rendering|Material|SetScalarParameterValue "/Game/Materials/MPC_ParameterCollection.MPC_ParameterCollection" "Chords_Stem" _returnvalue :!class /Script/Engine.KismetMaterialLibrary))

(event Custom|OnDrumsChanged
  (params (OutputName :type Name) (Output :type Meta%20Sound%20Output%20Structure%20%28by%20ref%29))
  (bind _returnvalue (Class|MetasoundOutputBlueprintAccess|GetFloat Output))
  (Rendering|Material|SetScalarParameterValue "/Game/Materials/MPC_ParameterCollection.MPC_ParameterCollection" "Drums_Stem" _returnvalue :!class /Script/Engine.KismetMaterialLibrary))

(event Custom|OnFXGameBoyChanged
  (params (OutputName :type Name) (Output :type Meta%20Sound%20Output%20Structure%20%28by%20ref%29))
  (bind _returnvalue (Class|MetasoundOutputBlueprintAccess|GetFloat Output))
  (Rendering|Material|SetScalarParameterValue "/Game/Materials/MPC_ParameterCollection.MPC_ParameterCollection" "FXGameBoy_Stem" _returnvalue :!class /Script/Engine.KismetMaterialLibrary))

(event Custom|OnFXGrowlsChanged
  (params (OutputName :type Name) (Output :type Meta%20Sound%20Output%20Structure%20%28by%20ref%29))
  (bind _returnvalue (Class|MetasoundOutputBlueprintAccess|GetFloat Output))
  (Rendering|Material|SetScalarParameterValue "/Game/Materials/MPC_ParameterCollection.MPC_ParameterCollection" "FXGrowls_Stem" _returnvalue :!class /Script/Engine.KismetMaterialLibrary))

(event Custom|OnLeadChanged
  (params (OutputName :type Name) (Output :type Meta%20Sound%20Output%20Structure%20%28by%20ref%29))
  (bind _returnvalue (Class|MetasoundOutputBlueprintAccess|GetFloat Output))
  (Rendering|Material|SetScalarParameterValue "/Game/Materials/MPC_ParameterCollection.MPC_ParameterCollection" "Lead_Stem" _returnvalue :!class /Script/Engine.KismetMaterialLibrary))

(event EventBeginPlay
  ;[0.15 0.15 0.15 0.5] 2.
  ; - "Create New Clock" node
  ; - set Clock Name
  ; - Drag off "In Settings" input (or Split Struct) and "Make Quartz Clock Settings"
  (bind _returnvalue (Class|QuartzSubsystem|CreateNewClock (WorldSubsystems|GetQuartzSubsystem) "Main" (Utilities|Struct|MakeQuartzClockSettings (Utilities|Struct|MakeQuartzTimeSignature 4 "QuarterNote" 0) false) false))
  ;[0.15 0.15 0.15 0.5] 3.
  ; Store as variable
  (bind _output_get (Variables|Default|SetQuartzClockHandle _returnvalue))
  ;[0.15 0.15 0.15 0.5] 4.
  ; - "Subsribe to Quantization Event"
  ; - Change Quantezation Enum
  ; - Drag off Red pin and make Custom Event
  (bind _clockhandle (Class|QuartzClockHandle|SubscribetoQuantizationEvent _output_get "QuarterNote" (delegate Custom|Beat)))
  ;[0.15 0.15 0.15 0.5] Set BPM
  (bind _clockhandle_2 (Class|QuartzClockHandle|SetBeatsPerMinute :self _clockhandle :BeatsPerMinute (Variables|Default|GetBPM%20Tempo)))
  (Utilities|FlowControl|Sequence
    (:then_0
      ;[0.15 0.15 0.15 0.5] Set Stem Driver Audio Component Up
      (if (Variables|Default|GetPlay%20Music)
        _))
    (:then_1
      ;[0.15 0.15 0.15 0.5] 7.
      ; - Start Clock
      (Utilities|FlowControl|Delay 1.0)
      (Class|QuartzClockHandle|StartClock _clockhandle_2)
      ;[0.15 0.15 0.15 0.5] Start Music Stems
      (if (Variables|Default|GetPlay%20Music)
        (CallFunction|StartMusic)))))

(event Collision|EventActorBeginOverlap
  (params (OtherActor :type Actor%20Object%20Reference)))

(event EventTick
  (params (DeltaSeconds :type Float%20%28single-precision%29))
  ;[0.15 0.15 0.15 0.5] Beat Progress Update
  (bind _returnvalue (Class|QuartzClockHandle|GetBeatProgressPercent (Variables|Default|GetQuartzClockHandle) "QuarterNote" 0.0 0.0))
  (Rendering|Material|SetScalarParameterValue "/Game/Materials/MPC_ParameterCollection.MPC_ParameterCollection" "Beat Percent" _returnvalue :!class /Script/Engine.KismetMaterialLibrary))

(fn ConstructionScript)
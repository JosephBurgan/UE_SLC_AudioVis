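; Beat manager actor that runs a Quartz clock to drive beat-synced audio and material parameters.
; On BeginPlay it creates the clock, subscribes to quarter-note events and starts it after a short delay.
; Each beat writes the beat number to a Material Parameter Collection and plays a MetaSound beep.
; Tick writes quarter-note progress to the same collection, giving materials a continuous phase.
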(event Custom|Beat
  (params (ClockName :type Name) (QuantizationType :type EQuartzCommandQuantization%20Enum :default "Bar") (NumBars :type Integer) (Beat :type Integer) (BeatFraction :type Float%20%28single-precision%29))
  ;[0.15 0.15 0.15 0.5] 4.
  ; - "Subsribe to Quantization Event"
  ; - Change Quantezation Enum
  ; - Drag off Red pin and make Custom Event
  ;[0.15 0.15 0.15 0.5] 5.
  ; - Make a Material Parameter Collection asset in the Content Browser
  ; - Add a Scalar Parameter and name it
  ; - Add this "Set Scalar Paramter Value" node
  ; - Set Collection as your Material Paramter Collection asset
  ; - Select the Parameter Name
  ; - Input the Beat Fraction
  (Rendering|Material|SetScalarParameterValue "/Game/Audio/MPC_ParameterCollection.MPC_ParameterCollection" "Beat" (Math|Conversions|ToFloat(Integer) Beat) :!class /Script/Engine.KismetMaterialLibrary)
  ;[0.15 0.15 0.15 0.5] 6.
  ; - Play MetaSound asset "BeepTone"
  (Audio|Components|Audio|Play (Variables|Default|GetAudioComponent%20MS_BeepTone) 0.0))

(event EventBeginPlay
  ;[0.15 0.15 0.15 0.5] 2.
  ; - "Create New Clock" node
  ; - set Clock Name
  ; - Drag off "In Settings" input (or Split Struct) and "Make Quartz Clock Settings"
  (bind _returnvalue (Class|QuartzSubsystem|CreateNewClock (WorldSubsystems|GetQuartzSubsystem) "Main" (Utilities|Struct|MakeQuartzClockSettings (Utilities|Struct|MakeQuartzTimeSignature 4 "QuarterNote" 0) false) false))
  ;[0.15 0.15 0.15 0.5] 3.
  ; Store as variable
  (bind _output_get (Variables|Default|SetQuartzClockHandle _returnvalue))
  ;[0.15 0.15 0.15 0.5] 4.
  ; - "Subsribe to Quantization Event"
  ; - Change Quantezation Enum
  ; - Drag off Red pin and make Custom Event
  (bind _clockhandle (Class|QuartzClockHandle|SubscribetoQuantizationEvent _output_get "QuarterNote" (delegate Custom|Beat)))
  ;[0.15 0.15 0.15 0.5] 7.
  ; - Start Clock
  (Utilities|FlowControl|Delay 1.0)
  (Class|QuartzClockHandle|StartClock _clockhandle))

(event Collision|EventActorBeginOverlap
  (params (OtherActor :type Actor%20Object%20Reference)))

(event EventTick
  (params (DeltaSeconds :type Float%20%28single-precision%29))
  ;[0.15 0.15 0.15 0.5] Beat Progress Update
  (bind _returnvalue (Class|QuartzClockHandle|GetBeatProgressPercent (Variables|Default|GetQuartzClockHandle) "QuarterNote" 0.0 0.0))
  (Rendering|Material|SetScalarParameterValue "/Game/Audio/MPC_ParameterCollection.MPC_ParameterCollection" "Beat Percent" _returnvalue :!class /Script/Engine.KismetMaterialLibrary))

(fn ConstructionScript)
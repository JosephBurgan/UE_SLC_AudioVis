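; BP_MIDI is an actor that plays an audio component, likely a MetaSound, live from a hardware MIDI input device.
; On BeginPlay it opens a controller for the device selected by the MIDIDevice index and binds note-on and note-off events.
; Note-on passes note and velocity as float parameters, fires a gate trigger, sets a held bool and prints debug text.
; Note-off clears the bool; an unconnected loop can print available devices.
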(event Custom|OnMIDINoteOn_Event
  (params (MIDIDeviceController :type MIDI%20Device%20Input%20Controller%20Object%20Reference) (Timestamp :type Integer) (Channel :type Integer) (Note :type Integer) (Velocity :type Integer))
  ;[0.15 0.15 0.15 0.5 30] Setup MIDI
  (Variables|Default|SetIn%20Bool true)
  (Audio|Parameter|SetFloatParameter (Variables|Default|GetAudioComponent%20-%20MS1) "MIDI Note" (Math|Conversions|ToFloat(Integer) Note) :!class /Script/AudioExtensions.AudioParameterControllerInterface)
  (Audio|Parameter|SetFloatParameter (Variables|Default|GetAudioComponent%20-%20MS1) "MIDI Velocity" (Math|Conversions|ToFloat(Integer) Velocity) :!class /Script/AudioExtensions.AudioParameterControllerInterface)
  (Class|AudioParameterControllerInterface|SetTriggerParameter (Variables|Default|GetAudioComponent%20-%20MS1) "MIDI Gate")
  (Effects|Components|ParticleSystem|SetBoolParameter (Variables|Default|GetAudioComponent%20-%20MS1) "MIDI Bool" (Variables|Default|GetIn%20Bool))
  (Development|PrintString (Utilities|String|Append "Note: " (Utilities|String|ToString(Integer) Note) " Velocity: " (Utilities|String|ToString(Integer) Velocity))))

(event Custom|Setup%20MIDI
  ;[0.15 0.15 0.15 0.5 30] Setup MIDI
  (Utilities|FlowControl|Sequence
    (:then_0)
    (:then_1
      (bind _outmididevices (Class|MIDIDeviceManager|FindMIDIDevices))
      (bind _returnvalue (Class|MIDIDeviceManager|CreateMIDIDeviceInputController (.deviceid (Utilities|Array|Get(acopy) _outmididevices (Variables|Default|GetMIDI%20Device))) 1024))
      (Variables|Default|SetMIDI%20Input%20Controller _returnvalue))
    (:then_2
      (EventDispatchers|AssignOnMIDINoteon (Variables|Default|GetMIDI%20Input%20Controller) (delegate Custom|OnMIDINoteOn_Event))
      (EventDispatchers|AssignOnMIDINoteOff (Variables|Default|GetMIDI%20Input%20Controller) (delegate Custom|OnMIDINoteOff_Event)))))

(event Custom|OnMIDINoteOff_Event
  (params (MIDIDeviceController :type MIDI%20Device%20Input%20Controller%20Object%20Reference) (Timestamp :type Integer) (Channel :type Integer) (Note :type Integer) (Velocity :type Integer))
  ;[0.15 0.15 0.15 0.5 30] Setup MIDI
  (Variables|Default|SetIn%20Bool false)
  (Effects|Components|ParticleSystem|SetBoolParameter (Variables|Default|GetAudioComponent%20-%20MS1) "MIDI Bool" (Variables|Default|GetIn%20Bool)))

(event EventBeginPlay
  (CallFunction|SetupMIDI))

(event Collision|EventActorBeginOverlap
  (params (OtherActor :type Actor%20Object%20Reference)))

(event EventTick
  (params (DeltaSeconds :type Float%20%28single-precision%29)))

(fn ConstructionScript)